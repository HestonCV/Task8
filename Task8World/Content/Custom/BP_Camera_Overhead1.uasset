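; Overhead orthographic camera that follows BP_Drone over a Cesium world, held at a fixed geographic height.
; Each tick it converts the drone's position through CesiumGeoreference to match longitude and latitude.
; Zoom events scale ortho width within min/max limits, while older height-based zoom logic is left unused.
; QueryBorderData traces from the four viewport corners and returns their longitude/latitude/height, printing any hit actor that isn't a Cesium tileset.
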(event Custom|ZoomOut
  (bind _camera (Variables|Default|GetCamera))
  (bind _orthowidth (Variables|/Script/Engine.CameraComponent|GetOrthoWidth _camera))
  (bind _returnvalue (* _orthowidth 1.25))
  ;[1 1 1] Zoom Out
  (if (>= _returnvalue (Variables|Default|GetMaxOrthoWidth))
    (Class|CameraComponent|SetOrthoWidth _camera (Math|Conversions|ToFloat(Integer) (Variables|Default|GetMaxOrthoWidth)))
    (else
      (Class|CameraComponent|SetOrthoWidth _camera _returnvalue))))

(event Custom|ZoomIn
  (bind _camera (Variables|Default|GetCamera))
  (bind _orthowidth (Variables|/Script/Engine.CameraComponent|GetOrthoWidth _camera))
  (bind _returnvalue (* _orthowidth 0.8))
  ;[1 1 1] Zoom In
  (if (<= _returnvalue (Variables|Default|GetMinOrthoWidth))
    (Class|CameraComponent|SetOrthoWidth _camera (Math|Conversions|ToFloat(Integer) (Variables|Default|GetMinOrthoWidth)))
    (else
      (Class|CameraComponent|SetOrthoWidth _camera _returnvalue))))

(event EventBeginPlay
  ;[1 1 1] Set input mode, orthowidth, and chosen UI
  (Class|CameraComponent|SetOrthoWidth (Variables|Default|GetCamera) (Math|Conversions|ToFloat(Integer) (Variables|Default|GetMinOrthoWidth))))

(event EventTick
  (params (DeltaSeconds :type Float%20%28single-precision%29))
  ;[1 1 1] Track Drone
  (bind _returnvalue (Actor|GetActorOfClass "/Script/CesiumRuntime.CesiumGeoreference"))
  (bind _returnvalue_2 (Actor|GetActorOfClass "/Game/Custom/BP_Drone.BP_Drone_C"))
  (Transformation|SetWorldLocation (Variables|Default|GetDefaultSceneRoot) (Class|CesiumGeoreference|TransformLongitudeLatitudeHeightPositiontoUnreal _returnvalue (Math|Vector|MakeVector (.X (Math|Vector|BreakVector (Class|CesiumGeoreference|TransformUnrealPositiontoLongitudeLatitudeHeight _returnvalue (Transformation|GetWorldLocation (Variables|/Script/Engine.Actor|GetRootComponent _returnvalue_2))))) (.Y (Math|Vector|BreakVector (Class|CesiumGeoreference|TransformUnrealPositiontoLongitudeLatitudeHeight _returnvalue (Transformation|GetWorldLocation (Variables|/Script/Engine.Actor|GetRootComponent _returnvalue_2))))) 7e+02)) false false))

(fn ConstructionScript)

(fn QueryBorderData
  (bind _returnvalue (Viewport|GetViewportSize))
  (bind _returnvalue_2 (Math|Vector2D|MakeVector2D 0.0 0.0))
  (bind _returnvalue_3 (Viewport|GetViewportSize))
  (bind _returnvalue_4 (Viewport|GetViewportSize))
  (bind _playerstate (Variables|GetPlayerState))
  (bind _playerstate_2 (Variables|GetPlayerState))
  (bind _playerstate_3 (Variables|GetPlayerState))
  (bind _playerstate_4 (Variables|GetPlayerState))
  (bind _y (Math|Vector2D|BreakVector2D _returnvalue))
  (bind _returnvalue_5 (Game|GetPlayerController _playerstate))
  (bind _returnvalue_6 (Game|GetPlayerController _playerstate_2))
  (bind _x (Math|Vector2D|BreakVector2D _returnvalue_3))
  (bind _returnvalue_7 (Game|GetPlayerController _playerstate_3))
  (bind (_x_2 _y_2) (Math|Vector2D|BreakVector2D _returnvalue_4))
  (bind _returnvalue_8 (Game|GetPlayerController _playerstate_4))
  (bind _returnvalue_9 (Math|Vector2D|MakeVector2D 0.0 _y))
  (bind _worldposition (Class|GameplayStatics|DeprojectScreentoWorld _returnvalue_6 _returnvalue_2))
  (bind _returnvalue_10 (Math|Vector2D|MakeVector2D _x 0.0))
  (bind _returnvalue_11 (Math|Vector2D|MakeVector2D _x_2 _y_2))
  (bind _worldposition_2 (Class|GameplayStatics|DeprojectScreentoWorld _returnvalue_5 _returnvalue_9))
  (bind _worldposition_3 (Class|GameplayStatics|DeprojectScreentoWorld _returnvalue_7 _returnvalue_10))
  (bind _worldposition_4 (Class|GameplayStatics|DeprojectScreentoWorld _returnvalue_8 _returnvalue_11))
  (bind _outhit (Collision|LineTraceByChannel _worldposition (+ _worldposition (* (Math|Vector|GetForwardVector (Variables|Default|GetCamera)) "1000000.000000,1000000.000000,1000000.000000")) "TraceTypeQuery1" false 0 "Persistent"))
  (Utilities|Casting|CastToCesium3DTileset (.HitActor (Collision|BreakHitResult _outhit))
    (:then
      _)
    (:CastFailed
      (Development|PrintString (Utilities|GetDisplayName (.HitActor (Collision|BreakHitResult _outhit))))))
  (bind _returnvalue_12 (Actor|GetActorOfClass "/Script/CesiumRuntime.CesiumGeoreference"))
  (Variables|Default|SetTopLeftCoord (Class|CesiumGeoreference|TransformUnrealPositiontoLongitudeLatitudeHeight _returnvalue_12 (.Location (Collision|BreakHitResult _outhit))))
  (bind _outhit_2 (Collision|LineTraceByChannel _worldposition_3 (+ _worldposition_3 (* (Math|Vector|GetForwardVector (Variables|Default|GetCamera)) "1000000.000000,1000000.000000,1000000.000000")) "TraceTypeQuery1" false 0 "Persistent"))
  (Utilities|Casting|CastToCesium3DTileset (.HitActor (Collision|BreakHitResult _outhit_2))
    (:then
      _)
    (:CastFailed
      (Development|PrintString (Utilities|GetDisplayName (.HitActor (Collision|BreakHitResult _outhit_2))))))
  (bind _returnvalue_13 (Actor|GetActorOfClass "/Script/CesiumRuntime.CesiumGeoreference"))
  (Variables|Default|SetTopRightCoord (Class|CesiumGeoreference|TransformUnrealPositiontoLongitudeLatitudeHeight _returnvalue_13 (.Location (Collision|BreakHitResult _outhit_2))))
  (bind _outhit_3 (Collision|LineTraceByChannel _worldposition_4 (+ _worldposition_4 (* (Math|Vector|GetForwardVector (Variables|Default|GetCamera)) "1000000.000000,1000000.000000,1000000.000000")) "TraceTypeQuery1" false 0 "Persistent"))
  (Utilities|Casting|CastToCesium3DTileset (.HitActor (Collision|BreakHitResult _outhit_3))
    (:then
      _)
    (:CastFailed
      (Development|PrintString (Utilities|GetDisplayName (.HitActor (Collision|BreakHitResult _outhit_3))))))
  (bind _returnvalue_14 (Actor|GetActorOfClass "/Script/CesiumRuntime.CesiumGeoreference"))
  (Variables|Default|SetBottomRightCoord (Class|CesiumGeoreference|TransformUnrealPositiontoLongitudeLatitudeHeight _returnvalue_14 (.Location (Collision|BreakHitResult _outhit_3))))
  (bind _outhit_4 (Collision|LineTraceByChannel _worldposition_2 (+ _worldposition_2 (* (Math|Vector|GetForwardVector (Variables|Default|GetCamera)) "1000000.000000,1000000.000000,1000000.000000")) "TraceTypeQuery1" false 0 "Persistent"))
  (Utilities|Casting|CastToCesium3DTileset (.HitActor (Collision|BreakHitResult _outhit_4))
    (:then
      _)
    (:CastFailed
      (Development|PrintString (Utilities|GetDisplayName (.HitActor (Collision|BreakHitResult _outhit_4))))))
  (bind _returnvalue_15 (Actor|GetActorOfClass "/Script/CesiumRuntime.CesiumGeoreference"))
  (Variables|Default|SetBottomLeftCoord (Class|CesiumGeoreference|TransformUnrealPositiontoLongitudeLatitudeHeight _returnvalue_15 (.Location (Collision|BreakHitResult _outhit_4))))
  (return (Variables|Default|GetTopLeftCoord) (Variables|Default|GetTopRightCoord) (Variables|Default|GetBottomRightCoord) (Variables|Default|GetBottomLeftCoord)))