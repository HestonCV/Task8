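; UI controller that manages switchable drone flight display designs and toggles the view between an overhead camera and the drone.
; ChangeUI disables the current widget and creates one of five designs, unless the drone view is active.
; UpdateUI forwards ownship, threat band and intruder data to the active widget, adding the overhead camera's border coordinates.
; ToggleCamera swaps view targets and toggles UI visibility, which can only be restored in overhead view.
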(event EventBeginPlay
  (bind _returnvalue (Actor|GetActorOfClass "/Game/Custom/BP_Camera_Overhead1.BP_Camera_Overhead1_C"))
  (bind _output_get (Variables|Default|SetOverhead _returnvalue))
  (Variables|Default|SetActiveCamera _output_get)
  (bind _returnvalue_2 (Actor|GetActorOfClass "/Game/Custom/BP_Drone.BP_Drone_C"))
  (Variables|Default|SetFOV _returnvalue_2))

(fn ConstructionScript)

(fn ChangeUI
  (params (Selection :type Integer))
  (bind _activecamera (Variables|Default|GetActiveCamera))
  (if (not (and (Utilities|IsValid _activecamera) (== _activecamera (Variables|Default|GetFOV))))
    (if (Utilities|IsValid (Variables|Default|GetActiveUIObject))
      (Default|Disable (Variables|Default|GetActiveUI)))
    (switch int Selection
      (:0
        (bind _returnvalue (UserInterface|CreateWidget "/Game/Custom/WBP_UIDesign_01.WBP_UIDesign_01_C"))
        (Variables|Default|SetActiveUI _returnvalue)
        (UserInterface|Viewport|AddtoViewport _returnvalue 0)
        (Variables|Default|SetActiveUIObject _returnvalue)
        (Default|Initialize _returnvalue))
      (:1
        (bind _returnvalue_2 (UserInterface|CreateWidget "/Game/Custom/WBP_UIDesign_02.WBP_UIDesign_02_C"))
        (Variables|Default|SetActiveUI _returnvalue_2)
        (UserInterface|Viewport|AddtoViewport _returnvalue_2 0)
        (Variables|Default|SetActiveUIObject _returnvalue_2)
        (Default|Initialize _returnvalue_2))
      (:2
        (bind _returnvalue_3 (UserInterface|CreateWidget "/Game/Custom/WBP_UIDesign_03.WBP_UIDesign_03_C"))
        (Variables|Default|SetActiveUI _returnvalue_3)
        (UserInterface|Viewport|AddtoViewport _returnvalue_3 0)
        (Variables|Default|SetActiveUIObject _returnvalue_3)
        (Default|Initialize _returnvalue_3))
      (:3
        (bind _returnvalue_4 (UserInterface|CreateWidget "/Game/Custom/WBP_UIDesign_04.WBP_UIDesign_04_C"))
        (Variables|Default|SetActiveUI _returnvalue_4)
        (UserInterface|Viewport|AddtoViewport _returnvalue_4 0)
        (Variables|Default|SetActiveUIObject _returnvalue_4)
        (Default|Initialize _returnvalue_4))
      (:4
        (bind _returnvalue_5 (UserInterface|CreateWidget "/Game/Custom/WBP_UIDesign_06.WBP_UIDesign_06_C"))
        (Variables|Default|SetActiveUI _returnvalue_5)
        (UserInterface|Viewport|AddtoViewport _returnvalue_5 0)
        (Variables|Default|SetActiveUIObject _returnvalue_5)
        (Default|Initialize _returnvalue_5)))))

(fn ToggleUI
  (bind _activeuiobject (Variables|Default|GetActiveUIObject))
  (if (Utilities|IsValid (Variables|Default|GetActiveUIObject))
    (if (Widget|IsVisible _activeuiobject)
      (Widget|SetVisibility _activeuiobject "Hidden")
      (else
        (Utilities|Casting|CastToBP_Camera_Overhead1 (Variables|Default|GetActiveCamera))
        (Widget|SetVisibility _activeuiobject "Visible")))))

(fn UpdateUI
  (params (OwnshipHeading :type Float%20%28double-precision%29) (OwnshipAltitude :type Float%20%28double-precision%29) (FlightTime :type Float%20%28double-precision%29) (ThreatBandStartAngle :type Float%20%28double-precision%29) (ThreatBandEndAngle :type Float%20%28double-precision%29) (ThreatBandThreatLevel :type Integer) (Intruders :type Array%20of%20BP%20Intruder%20Object%20References) (Debug :type Boolean))
  (if (Utilities|IsValid (Variables|Default|GetActiveUIObject))
    (bind (_topleftcoord _toprightcoord _bottomrightcoord _bottomleftcoord) (Default|QueryBorderData (Variables|Default|GetOverhead)))
    (Default|UpdateUI (Variables|Default|GetActiveUI) OwnshipHeading OwnshipAltitude FlightTime ThreatBandStartAngle ThreatBandEndAngle ThreatBandThreatLevel Intruders _topleftcoord _toprightcoord _bottomrightcoord _bottomleftcoord Debug)))

(fn ToggleCamera
  (bind _fov (Variables|Default|GetFOV))
  (bind _overhead (Variables|Default|GetOverhead))
  (Utilities|Casting|CastToBP_Camera_Overhead1 (Variables|Default|GetActiveCamera)
    (:then
      (Game|Player|SetViewTargetwithBlend (Game|GetPlayerController (Game|GetPlayerState 0)) _fov 0.0 "VTBlend_Linear" 0.0 false)
      (Variables|Default|SetActiveCamera _fov))
    (:CastFailed
      (Game|Player|SetViewTargetwithBlend (Game|GetPlayerController (Game|GetPlayerState 0)) _overhead 0.0 "VTBlend_Linear" 0.0 false)
      (Variables|Default|SetActiveCamera _overhead)))
  (CallFunction|ToggleUI))