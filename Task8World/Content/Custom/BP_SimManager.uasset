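; BP_SimManager runs a drone flight simulation, gathering ownship and intruder state and pushing it to the UI.
; BeginPlay finds the drone, intruders and UI controller, sets game-and-UI input, starts a one-second flight-time counter and plays a timed, scripted threat-band sequence.
; Each tick sends heading, Cesium-georeferenced altitude, flight time, threat band and a refreshed intruder list to BP_UIController.
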(event Custom|IncrementFlightTime
  ;[1 1 1] Seconds counter
  (Variables|Default|SetFlightTimeSeconds (+ (Variables|Default|GetFlightTimeSeconds) 1.0)))

(event EventBeginPlay
  ;[1 1 1] Set relevant components
  (bind _returnvalue (Actor|GetActorOfClass "/Game/Custom/BP_Drone.BP_Drone_C"))
  (Variables|Default|SetDrone _returnvalue)
  (bind _outactors (Actor|GetAllActorsOfClass "/Game/Custom/BP_Intruder.BP_Intruder_C"))
  (Variables|Default|SetIntruders _outactors)
  (bind _returnvalue_2 (Actor|GetActorOfClass "/Game/Custom/BP_UIController.BP_UIController_C"))
  (Variables|Default|SetUIController _returnvalue_2)
  (Input|SetInputModeGameandUI (Game|GetPlayerController 0) 0 "LockAlways" false false)
  (Default|ChangeUI (Variables|Default|GetUIController))
  (Utilities|Time|SetTimerbyEvent (delegate Custom|IncrementFlightTime) 1.0 true)
  (Utilities|FlowControl|Delay 4.0)
  (Variables|Default|SetThreatBandStartAngle 25.0)
  (Utilities|FlowControl|Delay 2.0)
  (Variables|Default|SetThreatBandStartAngle 35.0)
  (Variables|Default|SetThreatBandThreatLevel 1)
  (Utilities|FlowControl|Delay 2.0)
  (Variables|Default|SetThreatBandStartAngle 45.0)
  (Variables|Default|SetThreatBandEndAngle 65.0)
  (Utilities|FlowControl|Delay 2.0)
  (Variables|Default|SetThreatBandThreatLevel 0))

(event EventTick
  (params (DeltaSeconds :type Float%20%28single-precision%29))
  (bind _drone (Variables|Default|GetDrone))
  (bind _defaultsceneroot (Variables|/Game/Custom/BP_Drone.BP_Drone_C|GetDefaultSceneRoot _drone))
  ;[1 1 1] Obtain relevant data and send to UI
  (bind _outactors (Actor|GetAllActorsOfClass "/Game/Custom/BP_Intruder.BP_Intruder_C"))
  (bind _returnvalue (Actor|GetActorOfClass "/Script/CesiumRuntime.CesiumGeoreference"))
  (Default|UpdateUI (Variables|Default|GetUIController) (.Yaw (Math|Rotator|BreakRotator (Transformation|GetWorldRotation _defaultsceneroot))) (.Z (Math|Vector|BreakVector (Class|CesiumGeoreference|TransformUnrealPositiontoLongitudeLatitudeHeight _returnvalue (Transformation|GetWorldLocation _defaultsceneroot)))) (Variables|Default|GetFlightTimeSeconds) (Variables|Default|GetThreatBandStartAngle) (Variables|Default|GetThreatBandEndAngle) (Variables|Default|GetThreatBandThreatLevel) _outactors false))

(fn ConstructionScript)