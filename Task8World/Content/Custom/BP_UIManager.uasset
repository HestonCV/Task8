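; BP_UIManager is an actor that puts one of six WBP_Design widgets on screen by index.
; ChangeUI switches on Selection, creates the matching widget, stores it in ActiveUI and adds it to the viewport.
; It does not remove the previous widget, and the index mapping skips from Design_05 to Design_07.
; The event graph and construction script are empty, so ChangeUI holds all the logic.
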(event EventBeginPlay)

(event Collision|EventActorBeginOverlap
  (params (OtherActor :type Actor%20Object%20Reference)))

(event EventTick
  (params (DeltaSeconds :type Float%20%28single-precision%29)))

(fn ConstructionScript)

(fn ChangeUI
  (params (Selection :type Integer))
  (switch int Selection
    (:0
      (bind _returnvalue (UserInterface|CreateWidget "/Game/Custom/WBP_Design_01.WBP_Design_01_C"))
      (Variables|Default|SetActiveUI _returnvalue)
      (UserInterface|Viewport|AddtoViewport _returnvalue 0))
    (:1
      (bind _returnvalue_2 (UserInterface|CreateWidget "/Game/Custom/WBP_Design_02.WBP_Design_02_C"))
      (Variables|Default|SetActiveUI _returnvalue_2)
      (UserInterface|Viewport|AddtoViewport _returnvalue_2 0))
    (:2
      (bind _returnvalue_3 (UserInterface|CreateWidget "/Game/Custom/WBP_Design_03.WBP_Design_03_C"))
      (Variables|Default|SetActiveUI _returnvalue_3)
      (UserInterface|Viewport|AddtoViewport _returnvalue_3 0))
    (:3
      (bind _returnvalue_4 (UserInterface|CreateWidget "/Game/Custom/WBP_Design_04.WBP_Design_04_C"))
      (Variables|Default|SetActiveUI _returnvalue_4)
      (UserInterface|Viewport|AddtoViewport _returnvalue_4 0))
    (:4
      (bind _returnvalue_5 (UserInterface|CreateWidget "/Game/Custom/WBP_Design_05.WBP_Design_05_C"))
      (Variables|Default|SetActiveUI _returnvalue_5)
      (UserInterface|Viewport|AddtoViewport _returnvalue_5 0))
    (:5
      (bind _returnvalue_6 (UserInterface|CreateWidget "/Game/Custom/WBP_Design_07.WBP_Design_07_C"))
      (Variables|Default|SetActiveUI _returnvalue_6)
      (UserInterface|Viewport|AddtoViewport _returnvalue_6 0))))