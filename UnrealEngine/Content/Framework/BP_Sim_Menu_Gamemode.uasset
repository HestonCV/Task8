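; Game mode for the simulation menus that manages the player roster and shared state of the lobby.
; On the Lobby Menu level it registers each new menu controller, has it create the lobby menu and runs its initial setup.
; UpdateLobby rebuilds profiles from connected controllers and pushes names or the selected mode to each one, as flagged.
; Logout removes the leaving controller and refreshes everyone's name list.
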(event Custom|UpdateLobby
  (params (PlayerNames :type Boolean) (ModeNames :type Boolean))
  (if PlayerNames
    (Utilities|Array|Clear (Variables|Default|GetAll_PlayerProfiles))
    (for _array_element (Variables|Default|GetAll_ConnectedPlayers)
      (Utilities|Array|Add (Variables|Default|GetAll_PlayerProfiles) (Variables|/Game/Framework/BP_Sim_Menu_Controller.BP_Sim_Menu_Controller_C|GetPlayerprofile_info _array_element))))
  (for _array_element_2 (Variables|Default|GetAll_ConnectedPlayers)
    (if PlayerNames
      (Default|UpdatePlayerNames _array_element_2 (Variables|Default|GetAll_PlayerProfiles)))
    (if ModeNames
      (Default|UpdateLevelSelection _array_element_2 (Variables|Default|GetSelected%20Mode%20Name)))))

(event EventBeginPlay)

(event EventTick
  (params (DeltaSeconds :type Float%20%28single-precision%29)))

(event EventHandleStartingNewPlayer
  (params (NewPlayer :type Player%20Controller%20Object%20Reference))
  (bind _returnvalue (Game|GetCurrentLevelName true))
  (switch string _returnvalue
    (:Lobby_Menu
      (bind _asbp_sim_menu_controller (Utilities|Casting|CastToBP_Sim_Menu_Controller NewPlayer))
      (Utilities|Array|Add (Variables|Default|GetAll_ConnectedPlayers) _asbp_sim_menu_controller)
      (Default|CreateLobbyMenu _asbp_sim_menu_controller)
      (Default|InitialSetup _asbp_sim_menu_controller))))

(event EventOnLogout
  (params (ExitingController :type Controller%20Object%20Reference))
  (bind _asbp_sim_menu_controller (Utilities|Casting|CastToBP_Sim_Menu_Controller ExitingController))
  (Utilities|Array|RemoveItem (Variables|Default|GetAll_ConnectedPlayers) _asbp_sim_menu_controller)
  (CallFunction|UpdateLobby true false))

(fn ConstructionScript)