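; Player controller for the menu and session lobby, showing the lobby and load-screen widgets with UI-only input for the local player.
; InitialSetup loads or creates a saved player profile and passes it to ServerUpdateLobby, which has the menu game mode refresh the lobby.
; Update events push player names and mode selection into the lobby widget.
; Ending the client session destroys it and opens the main menu level.
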(event Custom|EndClientSession
  (|DestroySession self
    (:then
      (Game|OpenLevel(byName) "Main_Menu"))))

(event Custom|CreateLobbyMenu
  (CallFunction|UIShowLobbyMenu))

(event Custom|InitialSetup
  (CallFunction|LoadSavedProfile)
  (CallFunction|ServerUpdateLobby (Variables|Default|GetPlayerprofile_info)))

(event Custom|UpdatePlayerNames
  (params (PlayerProfiles :type Array%20of%20S%20Player%20Profile%20Structures))
  (bind _w_lobbymenu (Variables|Default|GetW_LobbyMenu))
  (Utilities|IsValid _w_lobbymenu
    (:Is%20Valid
      (Default|ClearPlayerNames _w_lobbymenu)
      (Default|UpdatePlayerNames _w_lobbymenu PlayerProfiles))))

(event Custom|ServerUpdateLobby
  (params (PlayerProfile :type S%20Player%20Profile%20Structure))
  (Variables|Default|SetPlayerprofile_info PlayerProfile)
  (bind _asbp_sim_menu_gamemode (Utilities|Casting|CastToBP_Sim_Menu_Gamemode (Game|GetGameMode)))
  (Default|UpdateLobby _asbp_sim_menu_gamemode true true))

(event Custom|CreateLoadScreen
  (CallFunction|UIShowLoadScreen))

(event Custom|UpdateLevelSelection
  (params (ModeRowName :type Name))
  (bind _w_lobbymenu (Variables|Default|GetW_LobbyMenu))
  (Utilities|IsValid _w_lobbymenu
    (:Is%20Valid
      (Default|UpdateModeSelection _w_lobbymenu ModeRowName))))

(event EventBeginPlay
  (if (Pawn|IsLocalController)
    (Variables|Default|SetbShowMouseCursor true)
    (Input|SetInputModeUIOnly self 0 "DoNotLock" false)))

(event EventTick
  (params (DeltaSeconds :type Float%20%28single-precision%29)))

(fn ConstructionScript)

(fn UIShowLobbyMenu
  (Utilities|IsValid (Variables|Default|GetW_LobbyMenu)
    (:Is%20Valid
      _)
    (:Is%20Not%20Valid
      (bind _returnvalue (UserInterface|CreateWidget "/Game/widgets/W_Lobby_Menu.W_Lobby_Menu_C" self))
      (Variables|Default|SetW_LobbyMenu _returnvalue)))
  (UserInterface|Viewport|AddtoViewport (Variables|Default|GetW_LobbyMenu) 0)
  (return))

(fn LoadSavedProfile
  (bind _returnvalue (SaveGame|DoesSaveGameExist (LocalVariables|GetLocal%20SlotName)))
  (if _returnvalue
    _
    (else
      (bind _returnvalue_2 (SaveGame|CreateSaveGameObject "/Game/SavedData/SG_Playerprofile.SG_Playerprofile_C"))
      (SaveGame|SaveGametoSlot _returnvalue_2 (LocalVariables|GetLocal%20SlotName))))
  (bind _returnvalue_3 (SaveGame|LoadGamefromSlot (LocalVariables|GetLocal%20SlotName)))
  (bind _assg_playerprofile (Utilities|Casting|CastToSG_Playerprofile _returnvalue_3))
  (Variables|Default|SetPlayerprofile_info (Variables|/Game/SavedData/SG_Playerprofile.SG_Playerprofile_C|GetPlayerprofile _assg_playerprofile))
  (return))

(fn UIShowLoadScreen
  (Viewport|RemoveAllWidgets)
  (Utilities|IsValid (Variables|Default|GetW_LoadScreen)
    (:Is%20Valid
      _)
    (:Is%20Not%20Valid
      (bind _returnvalue (UserInterface|CreateWidget "/Game/widgets/W_Load_Screen.W_Load_Screen_C" self))
      (Variables|Default|SetW_LoadScreen _returnvalue)))
  (UserInterface|Viewport|AddtoViewport (Variables|Default|GetW_LoadScreen) 0)
  (return))