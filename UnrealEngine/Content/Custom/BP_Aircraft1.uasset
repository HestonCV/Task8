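; Ownship aircraft that replays flight data on a Cesium globe and feeds the flight UI.
; Update lerps longitude/latitude/height via a timeline, then requests the GM's next row; Heading and Pitch are unused.
; Once activated, Tick holds PilotCamera downward-facing at fixed height, sending flight stats, intruders, a hardcoded threat band and screen-corner trace coordinates to BP_UIController.
; SwitchCamera toggles pilot/orbit cameras and the UI.
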(event Custom|Activate
  (Variables|Default|SetIsActive true)
  (bind _returnvalue (Actor|GetActorOfClass "/Game/Custom/BP_UIController.BP_UIController_C"))
  (bind _output_get (Variables|Default|SetUIController _returnvalue))
  (Default|SetUI _output_get)
  (Transformation|DetachFromComponent (Variables|Default|GetPilotCamera) "KeepWorld" "KeepWorld" "KeepWorld" true)
  (Transformation|SetWorldRotation (Variables|Default|GetPilotCamera) "-90.000000,-90.000000,0.000000" false false)
  (Variables|/Script/Engine.SceneCaptureComponent2D|SetTextureTarget (Variables|Default|GetSceneCaptureComponent2D) "/Game/Custom/FOV/CameraViewRenderTarget.CameraViewRenderTarget"))

(event Custom|Update
  (params (LongLatHeight :type Vector) (FlightTime :type Float%20%28double-precision%29) (Speed :type Float%20%28double-precision%29) (Heading :type Float%20%28double-precision%29) (Pitch :type Float%20%28double-precision%29))
  (Variables|Default|SetFlightTime FlightTime)
  (Variables|Default|SetSpeed Speed)
  (Variables|Default|SetAltitude (.Z (Math|Vector|BreakVector (Variables|Default|GetLastLongLatHeight))))
  (bind _returnvalue (Actor|GetActorOfClass "/Script/CesiumRuntime.CesiumGeoreference"))
  (if (not (Class|KismetMathLibrary|EqualExactlyVectorVector (Variables|Default|GetLastLongLatHeight) "0, 0, 0"))
    (bind _location (Timeline|Timeline PlayFromStart)
      (:Update
        (Transformation|SetWorldLocation (Variables|Default|GetRoot) (Class|CesiumGeoreference|TransformLongitudeLatitudeHeightPositiontoUnreal _returnvalue (Math|Vector|Lerp(Vector) (Variables|Default|GetLastLongLatHeight) LongLatHeight _location)) false false))
      (:Finished
        (Variables|Default|SetLastLongLatHeight LongLatHeight)
        (bind _asgm (Utilities|Casting|CastToGM (Game|GetGameMode)))
        (Default|GetNextRow _asgm)))
    (else
      (Transformation|SetWorldLocation (Variables|Default|GetRoot) (Class|CesiumGeoreference|TransformLongitudeLatitudeHeightPositiontoUnreal _returnvalue LongLatHeight) false false)
      (Variables|Default|SetLastLongLatHeight LongLatHeight)
      (bind _asgm_2 (Utilities|Casting|CastToGM (Game|GetGameMode)))
      (Default|GetNextRow _asgm_2))))

(event EventTick
  (params (DeltaSeconds :type Float%20%28single-precision%29))
  (if (Variables|Default|GetIsActive)
    (bind _returnvalue (Actor|GetActorOfClass "/Script/CesiumRuntime.CesiumGeoreference"))
    (Transformation|SetWorldLocation (Variables|Default|GetPilotCamera) (Class|CesiumGeoreference|TransformLongitudeLatitudeHeightPositiontoUnreal _returnvalue (Math|Vector|MakeVector (.X (Math|Vector|BreakVector (Class|CesiumGeoreference|TransformUnrealPositiontoLongitudeLatitudeHeight _returnvalue (Transformation|GetWorldLocation (Variables|Default|GetRoot))))) (.Y (Math|Vector|BreakVector (Class|CesiumGeoreference|TransformUnrealPositiontoLongitudeLatitudeHeight _returnvalue (Transformation|GetWorldLocation (Variables|Default|GetRoot))))) 1.6e+03)) false false)
    (Transformation|SetWorldRotation (Variables|Default|GetPilotCamera) (Class|CesiumGeoreference|TransformEastSouthUpRotatortoUnreal _returnvalue (Math|Rotator|MakeRotator 0.0 -9e+01 -9e+01) (Class|CesiumGeoreference|TransformLongitudeLatitudeHeightPositiontoUnreal _returnvalue (Math|Vector|MakeVector (.X (Math|Vector|BreakVector (Class|CesiumGeoreference|TransformUnrealPositiontoLongitudeLatitudeHeight _returnvalue (Transformation|GetWorldLocation (Variables|Default|GetRoot))))) (.Y (Math|Vector|BreakVector (Class|CesiumGeoreference|TransformUnrealPositiontoLongitudeLatitudeHeight _returnvalue (Transformation|GetWorldLocation (Variables|Default|GetRoot))))) 1.6e+03))) false false)
    (bind _outactors (Actor|GetAllActorsOfClass "/Game/Custom/BP_Intruder.BP_Intruder_C"))
    (bind (_topleftcoord _toprightcoord _bottomrightcoord _bottomleftcoord) (CallFunction|GetCameraBorderData))
    (Default|UpdateUI (Variables|Default|GetUIController) 0.0 (Variables|Default|GetAltitude) (Variables|Default|GetSpeed) 0.0 0.0 (Variables|Default|GetFlightTime) 275.0 3e+02 1 _outactors _topleftcoord _toprightcoord _bottomrightcoord _bottomleftcoord true)))

(event Input|ActionEvents|InputActionSwitchCamera
  (params (Key :type Key%20Structure :default "None"))
  (:Pressed
    (Utilities|FlowControl|FlipFlop
      (:A
        (Components|Activation|SetActive (Variables|Default|GetOrbitCamera) false false)
        (Components|Activation|SetActive (Variables|Default|GetPilotCamera) true false))
      (:B
        (Components|Activation|SetActive (Variables|Default|GetPilotCamera) false false)
        (Components|Activation|SetActive (Variables|Default|GetOrbitCamera) true false)))
    (Default|ToggleUI (Variables|Default|GetUIController))))

(fn ConstructionScript)

(fn GetCameraBorderData
  (bind _returnvalue (Game|GetPlayerController 0))
  (bind _returnvalue_2 (Game|GetPlayerController 0))
  (bind _returnvalue_3 (Viewport|GetViewportSize))
  (bind _returnvalue_4 (Math|Vector2D|MakeVector2D 0.0 0.0))
  (bind _returnvalue_5 (Viewport|GetViewportSize))
  (bind _returnvalue_6 (Viewport|GetViewportSize))
  (bind _returnvalue_7 (Game|GetPlayerController 0))
  (bind _returnvalue_8 (Game|GetPlayerController 0))
  (bind _y (Math|Vector2D|BreakVector2D _returnvalue_3))
  (bind _worldposition (Class|GameplayStatics|DeprojectScreentoWorld _returnvalue_8 _returnvalue_4))
  (bind _x (Math|Vector2D|BreakVector2D _returnvalue_5))
  (bind (_x_2 _y_2) (Math|Vector2D|BreakVector2D _returnvalue_6))
  (bind _returnvalue_9 (Math|Vector2D|MakeVector2D 0.0 _y))
  (bind _returnvalue_10 (Math|Vector2D|MakeVector2D _x 0.0))
  (bind _returnvalue_11 (Math|Vector2D|MakeVector2D _x_2 _y_2))
  (bind _worldposition_2 (Class|GameplayStatics|DeprojectScreentoWorld _returnvalue_7 _returnvalue_9))
  (bind _worldposition_3 (Class|GameplayStatics|DeprojectScreentoWorld _returnvalue _returnvalue_10))
  (bind _worldposition_4 (Class|GameplayStatics|DeprojectScreentoWorld _returnvalue_2 _returnvalue_11))
  (bind _outhit (Collision|LineTraceByChannel _worldposition (+ _worldposition (* (Math|Vector|GetForwardVector (Variables|Default|GetPilotCamera)) "1000000.000000,1000000.000000,1000000.000000")) "TraceTypeQuery1" false 0 "None"))
  (Utilities|Casting|CastToCesium3DTileset (.HitActor (Collision|BreakHitResult _outhit))
    (:then
      _)
    (:CastFailed
      _))
  (bind _returnvalue_12 (Actor|GetActorOfClass "/Script/CesiumRuntime.CesiumGeoreference"))
  (Variables|Default|SetTopLeftCoord (Class|CesiumGeoreference|TransformUnrealPositiontoLongitudeLatitudeHeight _returnvalue_12 (.Location (Collision|BreakHitResult _outhit))))
  (bind _outhit_2 (Collision|LineTraceByChannel _worldposition_3 (+ _worldposition_3 (* (Math|Vector|GetForwardVector (Variables|Default|GetPilotCamera)) "1000000.000000,1000000.000000,1000000.000000")) "TraceTypeQuery1" false 0 "None"))
  (Utilities|Casting|CastToCesium3DTileset (.HitActor (Collision|BreakHitResult _outhit_2))
    (:then
      _)
    (:CastFailed
      _))
  (bind _returnvalue_13 (Actor|GetActorOfClass "/Script/CesiumRuntime.CesiumGeoreference"))
  (Variables|Default|SetTopRightCoord (Class|CesiumGeoreference|TransformUnrealPositiontoLongitudeLatitudeHeight _returnvalue_13 (.Location (Collision|BreakHitResult _outhit_2))))
  (bind _outhit_3 (Collision|LineTraceByChannel _worldposition_4 (+ _worldposition_4 (* (Math|Vector|GetForwardVector (Variables|Default|GetPilotCamera)) "1000000.000000,1000000.000000,1000000.000000")) "TraceTypeQuery1" false 0 "None"))
  (Utilities|Casting|CastToCesium3DTileset (.HitActor (Collision|BreakHitResult _outhit_3))
    (:then
      _)
    (:CastFailed
      _))
  (bind _returnvalue_14 (Actor|GetActorOfClass "/Script/CesiumRuntime.CesiumGeoreference"))
  (Variables|Default|SetBottomRightCoord (Class|CesiumGeoreference|TransformUnrealPositiontoLongitudeLatitudeHeight _returnvalue_14 (.Location (Collision|BreakHitResult _outhit_3))))
  (bind _outhit_4 (Collision|LineTraceByChannel _worldposition_2 (+ _worldposition_2 (* (Math|Vector|GetForwardVector (Variables|Default|GetPilotCamera)) "1000000.000000,1000000.000000,1000000.000000")) "TraceTypeQuery1" false 0 "None"))
  (Utilities|Casting|CastToCesium3DTileset (.HitActor (Collision|BreakHitResult _outhit_4))
    (:then
      _)
    (:CastFailed
      _))
  (bind _returnvalue_15 (Actor|GetActorOfClass "/Script/CesiumRuntime.CesiumGeoreference"))
  (Variables|Default|SetBottomLeftCoord (Class|CesiumGeoreference|TransformUnrealPositiontoLongitudeLatitudeHeight _returnvalue_15 (.Location (Collision|BreakHitResult _outhit_4))))
  (return (Variables|Default|GetTopLeftCoord) (Variables|Default|GetTopRightCoord) (Variables|Default|GetBottomRightCoord) (Variables|Default|GetBottomLeftCoord)))