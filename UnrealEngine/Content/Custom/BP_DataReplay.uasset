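; Ownship actor that replays recorded flight data from a data table on a Cesium georeferenced globe.
; A timeline interpolates position, attitude, speed and time between rows at timestamp-scaled rates; Tick places the aircraft and top-down camera.
; Screen-corner traces give geographic view bounds to the UI controller on a timer and every frame.
; Keys switch cameras, scrub ownship or intruder rows, and zoom iteratively toward mile diameters measured by haversine.
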(event Custom|Zoom
  (params (Diameter%28Miles%29 :type Float%20%28double-precision%29))
  (bind _distance_miles_ (CallFunction|GetCircleDiameter(Miles)))
  (bind _returnvalue (Math|Vector2D|MakeVector2D Diameter%28Miles%29 0.0))
  (bind _pilotcamera (Variables|Default|GetPilotCamera))
  (bind _pilotcamera_2 (Variables|Default|GetPilotCamera))
  (bind _returnvalue_2 (Math|Vector2D|MakeVector2D _distance_miles_ 0.0))
  (bind _returnvalue_3 (Math|Vector|Distance2D(Vector) _returnvalue_2 _returnvalue))
  (if (not (Math|Float|NearlyEqual(Float) _distance_miles_ Diameter%28Miles%29 0.01)) :!label _label
    (if (< _returnvalue_3 0.1)
      (Variables|Default|SetZoomMagnitude 2e+01)
      (elif (> _returnvalue_3 1.0)
        (Variables|Default|SetZoomMagnitude 4.5e+02)
        (else
          (Variables|Default|SetZoomMagnitude 2e+02))))
    (if (< (CallFunction|GetCircleDiameter(Miles)) Diameter%28Miles%29)
      (Class|CameraComponent|SetOrthoWidth _pilotcamera_2 (+ (Variables|/Script/Engine.CameraComponent|GetOrthoWidth _pilotcamera_2) (* 1.2e+03 (Variables|Default|GetZoomMagnitude))))
      (Variables|Default|SetCameraHeight (+ (Variables|Default|GetCameraHeight) (* (Variables|Default|GetZoomMagnitude) 9.0)))
      (else
        (Class|CameraComponent|SetOrthoWidth _pilotcamera (+ (Variables|/Script/Engine.CameraComponent|GetOrthoWidth _pilotcamera) (* -1.2e+03 (Variables|Default|GetZoomMagnitude))))
        (Variables|Default|SetCameraHeight (+ (Variables|Default|GetCameraHeight) (* (Variables|Default|GetZoomMagnitude) -9.0)))))
    (Utilities|FlowControl|Delay 0.0)
    (goto _label)))

(event Custom|Activate
  (params (OwnshipTable :type Data%20Table%20Object%20Reference) (UIController :type BP%20UI%20Controller%20Object%20Reference) (RefreshRate :type Float%20%28double-precision%29))
  ;[1 1 1] Begin Update Loop and Refresh Timer
  (Variables|Default|SetIsActive true)
  (Variables|Default|SetOwnshipTable OwnshipTable)
  (Variables|Default|SetUIController UIController)
  (Transformation|DetachFromComponent (Variables|Default|GetPilotCamera) "KeepWorld" "KeepWorld" "KeepWorld" true)
  (Transformation|SetWorldRotation (Variables|Default|GetPilotCamera) "-90.000000,-90.000000,0.000000" false false)
  (Variables|/Script/Engine.SceneCaptureComponent2D|SetTextureTarget (Variables|Default|GetSceneCaptureComponent2D) "/Game/Custom/FOV/CameraViewRenderTarget.CameraViewRenderTarget")
  (Utilities|Time|SetTimerbyEvent (delegate Custom|UpdateUI) RefreshRate true)
  (CallFunction|UpdateLoop (Variables|Default|GetCurrentRow)))

(event Custom|UpdateLoop
  (params (Index :type Integer))
  (bind _ownshiptable (Variables|Default|GetOwnshipTable))
  ;[1 1 1] Update values to data from table using linear interpolation
  (bind _outrownames (DataTable|GetDataTableRowNames _ownshiptable))
  (if (>= (Utilities|Array|LastIndex _outrownames) Index)
    (bind _returnvalue (Utilities|GetDataTableRow _ownshiptable (Utilities|String|StringToName (Utilities|String|ToString(Integer) Index)))
      (:then
        (if (> (.timestamp_delta (Utilities|Struct|BreakStructure_Ownship _returnvalue)) 0)
          (Components|Timeline|SetPlayRate (Variables|Default|GetTimeline) (Math|Conversions|ToFloat(Integer) (/ 1000 (.timestamp_delta (Utilities|Struct|BreakStructure_Ownship _returnvalue)))))
          (bind _newtrack_0 (Timeline|Timeline PlayFromStart)
            (:Update
              (Variables|Default|SetCurrentFlightTime (Math|Float|Lerp (Variables|Default|GetLastFlightTime) (/ (Math|Conversions|ToFloat(Integer) (.timestamp (Utilities|Struct|BreakStructure_Ownship _returnvalue))) 1e+03) _newtrack_0))
              (Variables|Default|SetCurrentLongLatHeight (Math|Vector|Lerp(Vector) (Variables|Default|GetLastLongLatHeight) (Math|Vector|MakeVector (.lon_degrees (Utilities|Struct|BreakStructure_Ownship _returnvalue)) (.lat_degrees (Utilities|Struct|BreakStructure_Ownship _returnvalue)) (.altitude_feet (Utilities|Struct|BreakStructure_Ownship _returnvalue))) _newtrack_0))
              (Variables|Default|SetCurrentRollPitchYaw (Math|Rotator|Lerp(Rotator) (Variables|Default|GetLastRollPitchYaw) (Math|Rotator|MakeRotator (.roll_degrees (Utilities|Struct|BreakStructure_Ownship _returnvalue)) (.pitch_degrees (Utilities|Struct|BreakStructure_Ownship _returnvalue)) (- (.heading_degrees (Utilities|Struct|BreakStructure_Ownship _returnvalue)) 9e+01)) _newtrack_0 true))
              (Variables|Default|SetCurrentGroundSpeed (Math|Float|Lerp (Variables|Default|GetLastGroundSpeed) (.groundspeed_feet_per_second (Utilities|Struct|BreakStructure_Ownship _returnvalue)) _newtrack_0)))
            (:Finished
              ;;[1 1 1] Finished lerp -- set last values to current values and call update again
              (Variables|Default|SetLastLongLatHeight (Variables|Default|GetCurrentLongLatHeight))
              (Variables|Default|SetLastRollPitchYaw (Variables|Default|GetCurrentRollPitchYaw))
              (Variables|Default|SetLastGroundSpeed (Variables|Default|GetCurrentGroundSpeed))
              (Variables|Default|SetLastFlightTime (Variables|Default|GetCurrentFlightTime))
              (bind _result (Math|Integer|IncrementInt (Variables|Default|GetCurrentRow))
                (:%20%20
                  (CallFunction|UpdateLoop _result)))))
          (else
            ;;[1 1 1] Case for first loop -- No need to lerp, instantly set current and last values
            (bind _output_get (Variables|Default|SetCurrentLongLatHeight (Math|Vector|MakeVector (.lon_degrees (Utilities|Struct|BreakStructure_Ownship _returnvalue)) (.lat_degrees (Utilities|Struct|BreakStructure_Ownship _returnvalue)) (.altitude_feet (Utilities|Struct|BreakStructure_Ownship _returnvalue)))))
            (Variables|Default|SetLastLongLatHeight _output_get)
            (bind _output_get_2 (Variables|Default|SetCurrentRollPitchYaw (Math|Rotator|MakeRotator (.roll_degrees (Utilities|Struct|BreakStructure_Ownship _returnvalue)) (.pitch_degrees (Utilities|Struct|BreakStructure_Ownship _returnvalue)) (- (.heading_degrees (Utilities|Struct|BreakStructure_Ownship _returnvalue)) 9e+01))))
            (Variables|Default|SetLastRollPitchYaw _output_get_2)
            (bind _output_get_3 (Variables|Default|SetCurrentGroundSpeed (.groundspeed_feet_per_second (Utilities|Struct|BreakStructure_Ownship _returnvalue))))
            (Variables|Default|SetLastGroundSpeed _output_get_3)
            (bind _output_get_4 (Variables|Default|SetCurrentFlightTime (/ (Math|Conversions|ToFloat(Integer) (.timestamp (Utilities|Struct|BreakStructure_Ownship _returnvalue))) 1e+03)))
            (Variables|Default|SetLastFlightTime _output_get_4)
            (bind _result_2 (Math|Integer|IncrementInt (Variables|Default|GetCurrentRow))
              (:%20%20
                (CallFunction|UpdateLoop _result_2)))))))
    (else
      (Development|PrintString "End of ownship data"))))

(event Custom|UpdateUI
  (bind _currentrollpitchyaw (Variables|Default|GetCurrentRollPitchYaw))
  (bind _currentlonglatheight (Variables|Default|GetCurrentLongLatHeight))
  (bind (_roll _pitch _yaw) (Math|Rotator|BreakRotator _currentrollpitchyaw))
  (bind (_x _y _z) (Math|Vector|BreakVector _currentlonglatheight))
  ;[1 1 1] Update UI with current values based on refresh rate
  (bind (_topleftcoord _toprightcoord _bottomrightcoord _bottomleftcoord) (CallFunction|GetCameraBorderData))
  (Variables|Default|SetLastAltitude _z)
  (Default|UpdateUI (Variables|Default|GetUIController) (+ _yaw 9e+01) _x _y _z (Variables|Default|GetCurrentGroundSpeed) _roll _pitch (Variables|Default|GetCurrentFlightTime) 0 _topleftcoord _toprightcoord _bottomrightcoord _bottomleftcoord false false))

(event EventTick
  (params (DeltaSeconds :type Float%20%28single-precision%29))
  (bind _currentlonglatheight (Variables|Default|GetCurrentLongLatHeight))
  (bind (_x _y) (Math|Vector|BreakVector _currentlonglatheight))
  ;[1 1 1] Event tick used for continuous updates -- ownship and camera locations / rotations
  (if (Variables|Default|GetIsActive)
    (bind _returnvalue (Actor|GetActorOfClass "/Script/CesiumRuntime.CesiumGeoreference"))
    (Utilities|FlowControl|Sequence
      (:then_0
        ;;[1 1 1] Set Aircraft Location
        (Transformation|SetWorldLocation (Variables|Default|GetRoot) (Class|CesiumGeoreference|TransformLongitudeLatitudeHeightPositiontoUnreal _returnvalue (Variables|Default|GetCurrentLongLatHeight)) false false)
        (Transformation|SetWorldRotation (Variables|Default|GetRoot) (Class|CesiumGeoreference|TransformEastSouthUpRotatortoUnreal _returnvalue (Variables|Default|GetCurrentRollPitchYaw) (Class|CesiumGeoreference|TransformLongitudeLatitudeHeightPositiontoUnreal _returnvalue (Variables|Default|GetCurrentLongLatHeight))) false false))
      (:then_1
        ;;[1 1 1] Set Camera Location
        (Transformation|SetWorldLocation (Variables|Default|GetPilotCamera) (Class|CesiumGeoreference|TransformLongitudeLatitudeHeightPositiontoUnreal _returnvalue (Math|Vector|MakeVector _x _y (Variables|Default|GetCameraHeight))) false false)
        (Transformation|SetWorldRotation (Variables|Default|GetPilotCamera) (Class|CesiumGeoreference|TransformEastSouthUpRotatortoUnreal _returnvalue (Math|Rotator|MakeRotator 0.0 -9e+01 -9e+01) (Class|CesiumGeoreference|TransformLongitudeLatitudeHeightPositiontoUnreal _returnvalue (Math|Vector|MakeVector _x _y (Variables|Default|GetCameraHeight)))) false false))
      (:then_2
        ;;[1 1 1] Update Intruders to maintain position on screen
        (bind (_topleftcoord _toprightcoord _bottomrightcoord _bottomleftcoord) (CallFunction|GetCameraBorderData))
        (Default|UpdateUI (Variables|Default|GetUIController) -99999.0 0.0 0.0 (Variables|Default|GetLastAltitude) -99999.0 -99999.0 -99999.0 -99999.0 0 _topleftcoord _toprightcoord _bottomrightcoord _bottomleftcoord false true)))))

(event Input|ActionEvents|InputActionSwitchCamera
  (params (Key :type Key%20Structure :default "None"))
  ;[1 1 1] Controls
  (:Pressed
    (Utilities|FlowControl|FlipFlop
      (:A
        (Components|Activation|SetActive (Variables|Default|GetOrbitCamera) false false)
        (Components|Activation|SetActive (Variables|Default|GetPilotCamera) true false))
      (:B
        (Components|Activation|SetActive (Variables|Default|GetPilotCamera) false false)
        (Components|Activation|SetActive (Variables|Default|GetOrbitCamera) true false)))
    (Default|ToggleUI (Variables|Default|GetUIController))))

(event Input|MouseEvents|MouseWheelUp
  (params (Key :type Key%20Structure :default "None"))
  (bind _uicontroller (Variables|Default|GetUIController))
  (bind _intrudercontroller (Variables|/Game/Custom/BP_UIController.BP_UIController_C|GetIntruderController _uicontroller))
  ;[1 1 1] Controls
  (:Pressed
    (if (not (Variables|Default|GetIsShiftDown))
      (Math|Integer|IncrementInt (Variables|Default|GetCurrentRow))
      (elif (Utilities|IsValid _intrudercontroller)
        (Math|Integer|IncrementInt (Variables|/Game/Custom/BP_IntruderController.BP_IntruderController_C|GetCurrentRow _intrudercontroller))))))

(event Input|MouseEvents|MouseWheelDown
  (params (Key :type Key%20Structure :default "None"))
  (bind _uicontroller (Variables|Default|GetUIController))
  (bind _intrudercontroller (Variables|/Game/Custom/BP_UIController.BP_UIController_C|GetIntruderController _uicontroller))
  ;[1 1 1] Controls
  (:Pressed
    (if (not (Variables|Default|GetIsShiftDown))
      (Math|Integer|DecrementInt (Variables|Default|GetCurrentRow))
      (elif (Utilities|IsValid _intrudercontroller)
        (Math|Integer|DecrementInt (Variables|/Game/Custom/BP_IntruderController.BP_IntruderController_C|GetCurrentRow _intrudercontroller))))))

(event Input|KeyboardEvents|LeftShift
  (params (Key :type Key%20Structure :default "None"))
  ;[1 1 1] Controls
  (:Pressed
    (Variables|Default|SetIsShiftDown true))
  (:Released
    (Variables|Default|SetIsShiftDown false)))

(event Input|KeyboardEvents|1
  (params (Key :type Key%20Structure :default "None"))
  ;[1 1 1] Controls
  (:Pressed
    (CallFunction|Zoom 1.0)))

(event Input|KeyboardEvents|2
  (params (Key :type Key%20Structure :default "None"))
  ;[1 1 1] Controls
  (:Pressed
    (CallFunction|Zoom 2.0)))

(event Input|KeyboardEvents|5
  (params (Key :type Key%20Structure :default "None"))
  ;[1 1 1] Controls
  (:Pressed
    (CallFunction|Zoom 5.0)))

(event Input|KeyboardEvents|9
  (params (Key :type Key%20Structure :default "None"))
  ;[1 1 1] Controls
  (:Pressed
    (CallFunction|Zoom 9.0)))

(event Input|KeyboardEvents|3
  (params (Key :type Key%20Structure :default "None"))
  ;[1 1 1] Controls
  (:Pressed
    (CallFunction|Zoom 3.0)))

(event Input|KeyboardEvents|4
  (params (Key :type Key%20Structure :default "None"))
  ;[1 1 1] Controls
  (:Pressed
    (CallFunction|Zoom 4.0)))

(fn ConstructionScript)

(fn GetCameraBorderData
  (bind _returnvalue (Game|GetPlayerController 0))
  (bind _returnvalue_2 (Game|GetPlayerController 0))
  (bind _returnvalue_3 (Viewport|GetViewportSize))
  (bind _returnvalue_4 (Math|Vector2D|MakeVector2D 0.0 0.0))
  (bind _returnvalue_5 (Viewport|GetViewportSize))
  (bind _returnvalue_6 (Viewport|GetViewportSize))
  (bind _returnvalue_7 (Game|GetPlayerController 0))
  (bind _returnvalue_8 (Game|GetPlayerController 0))
  (bind _y (Math|Vector2D|BreakVector2D _returnvalue_3))
  (bind _worldposition (Class|GameplayStatics|DeprojectScreentoWorld _returnvalue_8 _returnvalue_4))
  (bind _x (Math|Vector2D|BreakVector2D _returnvalue_5))
  (bind (_x_2 _y_2) (Math|Vector2D|BreakVector2D _returnvalue_6))
  (bind _returnvalue_9 (Math|Vector2D|MakeVector2D 0.0 _y))
  (bind _returnvalue_10 (Math|Vector2D|MakeVector2D _x 0.0))
  (bind _returnvalue_11 (Math|Vector2D|MakeVector2D _x_2 _y_2))
  (bind _worldposition_2 (Class|GameplayStatics|DeprojectScreentoWorld _returnvalue_7 _returnvalue_9))
  (bind _worldposition_3 (Class|GameplayStatics|DeprojectScreentoWorld _returnvalue _returnvalue_10))
  (bind _worldposition_4 (Class|GameplayStatics|DeprojectScreentoWorld _returnvalue_2 _returnvalue_11))
  (bind _outhit (Collision|LineTraceByChannel _worldposition (+ _worldposition (* (Math|Vector|GetForwardVector (Variables|Default|GetPilotCamera)) "100000000.000000,100000000.000000,100000000.000000")) "TraceTypeQuery1" false 0 "None"))
  (Utilities|Casting|CastToCesium3DTileset (.HitActor (Collision|BreakHitResult _outhit))
    (:then
      _)
    (:CastFailed
      _))
  (bind _returnvalue_12 (Actor|GetActorOfClass "/Script/CesiumRuntime.CesiumGeoreference"))
  (Variables|Default|SetTopLeftCoord (Class|CesiumGeoreference|TransformUnrealPositiontoLongitudeLatitudeHeight _returnvalue_12 (.Location (Collision|BreakHitResult _outhit))))
  (bind _outhit_2 (Collision|LineTraceByChannel _worldposition_3 (+ _worldposition_3 (* (Math|Vector|GetForwardVector (Variables|Default|GetPilotCamera)) "100000000.000000,100000000.000000,100000000.000000")) "TraceTypeQuery1" false 0 "None"))
  (Utilities|Casting|CastToCesium3DTileset (.HitActor (Collision|BreakHitResult _outhit_2))
    (:then
      _)
    (:CastFailed
      _))
  (bind _returnvalue_13 (Actor|GetActorOfClass "/Script/CesiumRuntime.CesiumGeoreference"))
  (Variables|Default|SetTopRightCoord (Class|CesiumGeoreference|TransformUnrealPositiontoLongitudeLatitudeHeight _returnvalue_13 (.Location (Collision|BreakHitResult _outhit_2))))
  (bind _outhit_3 (Collision|LineTraceByChannel _worldposition_4 (+ _worldposition_4 (* (Math|Vector|GetForwardVector (Variables|Default|GetPilotCamera)) "100000000.000000,100000000.000000,100000000.000000")) "TraceTypeQuery1" false 0 "None"))
  (Utilities|Casting|CastToCesium3DTileset (.HitActor (Collision|BreakHitResult _outhit_3))
    (:then
      _)
    (:CastFailed
      _))
  (bind _returnvalue_14 (Actor|GetActorOfClass "/Script/CesiumRuntime.CesiumGeoreference"))
  (Variables|Default|SetBottomRightCoord (Class|CesiumGeoreference|TransformUnrealPositiontoLongitudeLatitudeHeight _returnvalue_14 (.Location (Collision|BreakHitResult _outhit_3))))
  (bind _outhit_4 (Collision|LineTraceByChannel _worldposition_2 (+ _worldposition_2 (* (Math|Vector|GetForwardVector (Variables|Default|GetPilotCamera)) "100000000.000000,100000000.000000,100000000.000000")) "TraceTypeQuery1" false 0 "None"))
  (Utilities|Casting|CastToCesium3DTileset (.HitActor (Collision|BreakHitResult _outhit_4))
    (:then
      _)
    (:CastFailed
      _))
  (bind _returnvalue_15 (Actor|GetActorOfClass "/Script/CesiumRuntime.CesiumGeoreference"))
  (Variables|Default|SetBottomLeftCoord (Class|CesiumGeoreference|TransformUnrealPositiontoLongitudeLatitudeHeight _returnvalue_15 (.Location (Collision|BreakHitResult _outhit_4))))
  (return (Variables|Default|GetTopLeftCoord) (Variables|Default|GetTopRightCoord) (Variables|Default|GetBottomRightCoord) (Variables|Default|GetBottomLeftCoord)))

(fn GetGroundHeight
  (bind _orbitcamera (Variables|Default|GetOrbitCamera))
  (bind _returnvalue (Transformation|GetWorldLocation _orbitcamera))
  (bind (_x _y _z) (Math|Vector|BreakVector _returnvalue))
  (bind _returnvalue_2 (+ _z 1e+03))
  (bind _returnvalue_3 (Math|Vector|MakeVector _x _y _returnvalue_2))
  (bind _outhit (Collision|LineTraceByChannel _returnvalue_3 (+ _returnvalue_3 (Math|Vector|MakeVector 0.0 0.0 -1e+05)) "TraceTypeQuery1" false 0 "None"))
  (Utilities|Casting|CastToCesium3DTileset (.HitActor (Collision|BreakHitResult _outhit))
    (:then
      _)
    (:CastFailed
      _))
  (bind _returnvalue_4 (Actor|GetActorOfClass "/Script/CesiumRuntime.CesiumGeoreference"))
  (return (+ (.Z (Math|Vector|BreakVector (Class|CesiumGeoreference|TransformUnrealPositiontoLongitudeLatitudeHeight _returnvalue_4 (.Location (Collision|BreakHitResult _outhit))))) 2.0)))

(fn GetCircleDiameter(Miles)
  (bind _returnvalue (Game|GetPlayerController 0))
  (bind _returnvalue_2 (Game|GetPlayerController 0))
  (bind _returnvalue_3 (Viewport|GetViewportSize))
  (bind _pilotcamera (Variables|Default|GetPilotCamera))
  (bind _returnvalue_4 (Math|Vector|GetForwardVector _pilotcamera))
  (bind _returnvalue_5 (/ _returnvalue_3 "(X=2.000000,Y=2.000000)"))
  (bind _returnvalue_6 (- _returnvalue_5 "(X=105.000000,Y=0.000000)"))
  (bind _returnvalue_7 (+ _returnvalue_5 "(X=105.000000,Y=0.000000)"))
  (bind _worldposition (Class|GameplayStatics|DeprojectScreentoWorld _returnvalue_2 _returnvalue_7))
  (bind _worldposition_2 (Class|GameplayStatics|DeprojectScreentoWorld _returnvalue _returnvalue_6))
  (Utilities|FlowControl|Sequence
    (:then_0
      ;[1 1 1] Left
      (bind _outhit (Collision|LineTraceByChannel _worldposition_2 (+ _worldposition_2 (* _returnvalue_4 "100000000.000000,100000000.000000,100000000.000000")) "TraceTypeQuery1" false 0 "Persistent" true "(R=0.000000,G=1.000000,B=0.928095,A=1.000000)")))
    (:then_1
      ;[1 1 1] Right
      (bind _outhit_2 (Collision|LineTraceByChannel _worldposition (+ _worldposition (* _returnvalue_4 "100000000.000000,100000000.000000,100000000.000000")) "TraceTypeQuery1" false 0 "Persistent")))
    (:then_2
      (bind _returnvalue_8 (Actor|GetActorOfClass "/Script/CesiumRuntime.CesiumGeoreference"))
      (return (* (* (Math|Trig|Atan2(Radians) (Math|Float|Sqrt (+ (* (Math|Trig|Cos(Radians) (Math|Trig|DegreesToRadians (.Y (Math|Vector|BreakVector (Class|CesiumGeoreference|TransformUnrealPositiontoLongitudeLatitudeHeight _returnvalue_8 (.Location (Collision|BreakHitResult _outhit))))))) (Math|Trig|Cos(Radians) (Math|Trig|DegreesToRadians (.Y (Math|Vector|BreakVector (Class|CesiumGeoreference|TransformUnrealPositiontoLongitudeLatitudeHeight _returnvalue_8 (.Location (Collision|BreakHitResult _outhit_2))))))) (Math|Float|Square (Math|Trig|Sin(Radians) (/ (- (Math|Trig|DegreesToRadians (.X (Math|Vector|BreakVector (Class|CesiumGeoreference|TransformUnrealPositiontoLongitudeLatitudeHeight _returnvalue_8 (.Location (Collision|BreakHitResult _outhit)))))) (Math|Trig|DegreesToRadians (.X (Math|Vector|BreakVector (Class|CesiumGeoreference|TransformUnrealPositiontoLongitudeLatitudeHeight _returnvalue_8 (.Location (Collision|BreakHitResult _outhit_2))))))) 2.0)))) (Math|Float|Square (Math|Trig|Sin(Radians) (/ (- (Math|Trig|DegreesToRadians (.Y (Math|Vector|BreakVector (Class|CesiumGeoreference|TransformUnrealPositiontoLongitudeLatitudeHeight _returnvalue_8 (.Location (Collision|BreakHitResult _outhit)))))) (Math|Trig|DegreesToRadians (.Y (Math|Vector|BreakVector (Class|CesiumGeoreference|TransformUnrealPositiontoLongitudeLatitudeHeight _returnvalue_8 (.Location (Collision|BreakHitResult _outhit_2))))))) 2.0))))) (Math|Float|Sqrt (- 1.0 (+ (* (Math|Trig|Cos(Radians) (Math|Trig|DegreesToRadians (.Y (Math|Vector|BreakVector (Class|CesiumGeoreference|TransformUnrealPositiontoLongitudeLatitudeHeight _returnvalue_8 (.Location (Collision|BreakHitResult _outhit))))))) (Math|Trig|Cos(Radians) (Math|Trig|DegreesToRadians (.Y (Math|Vector|BreakVector (Class|CesiumGeoreference|TransformUnrealPositiontoLongitudeLatitudeHeight _returnvalue_8 (.Location (Collision|BreakHitResult _outhit_2))))))) (Math|Float|Square (Math|Trig|Sin(Radians) (/ (- (Math|Trig|DegreesToRadians (.X (Math|Vector|BreakVector (Class|CesiumGeoreference|TransformUnrealPositiontoLongitudeLatitudeHeight _returnvalue_8 (.Location (Collision|BreakHitResult _outhit)))))) (Math|Trig|DegreesToRadians (.X (Math|Vector|BreakVector (Class|CesiumGeoreference|TransformUnrealPositiontoLongitudeLatitudeHeight _returnvalue_8 (.Location (Collision|BreakHitResult _outhit_2))))))) 2.0)))) (Math|Float|Square (Math|Trig|Sin(Radians) (/ (- (Math|Trig|DegreesToRadians (.Y (Math|Vector|BreakVector (Class|CesiumGeoreference|TransformUnrealPositiontoLongitudeLatitudeHeight _returnvalue_8 (.Location (Collision|BreakHitResult _outhit)))))) (Math|Trig|DegreesToRadians (.Y (Math|Vector|BreakVector (Class|CesiumGeoreference|TransformUnrealPositiontoLongitudeLatitudeHeight _returnvalue_8 (.Location (Collision|BreakHitResult _outhit_2))))))) 2.0))))))) 2.0) 3958.8)))))