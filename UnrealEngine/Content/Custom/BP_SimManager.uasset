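; BP_SimManager is the manager for a flight sim, feeding flight time, threat band and intruder data to the UI.
; BeginPlay caches the airliner, intruders and UI controller, sets game-and-UI input and starts a looping one-second flight timer.
; Tick re-queries all intruders and pushes them with the timer and threat band values to BP_UIController.
; A timed threat band test sequence and Cesium georeference conversions remain unconnected.
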(event Custom|IncrementFlightTime
  ;[1 1 1] Seconds counter
  (Variables|Default|SetFlightTimeSeconds (+ (Variables|Default|GetFlightTimeSeconds) 1.0)))

(event EventBeginPlay
  ;[1 1 1] Set relevant components
  (bind _returnvalue (Actor|GetActorOfClass "/Game/Blueprints/BP_Airliner.BP_Airliner_C"))
  (Variables|Default|SetDrone _returnvalue)
  (bind _outactors (Actor|GetAllActorsOfClass "/Game/Custom/BP_Intruder.BP_Intruder_C"))
  (Variables|Default|SetIntruders _outactors)
  (bind _returnvalue_2 (Actor|GetActorOfClass "/Game/Custom/BP_UIController.BP_UIController_C"))
  (Variables|Default|SetUIController _returnvalue_2)
  (Input|SetInputModeGameandUI (Game|GetPlayerController 0) 0 "LockAlways" false false)
  (Default|SetUI (Variables|Default|GetUIController))
  (Utilities|Time|SetTimerbyEvent (delegate Custom|IncrementFlightTime) 1.0 true))

(event EventTick
  (params (DeltaSeconds :type Float%20%28single-precision%29))
  ;[1 1 1] Obtain relevant data and send to UI
  (bind _outactors (Actor|GetAllActorsOfClass "/Game/Custom/BP_Intruder.BP_Intruder_C"))
  (bind _returnvalue (Actor|GetActorOfClass "/Script/CesiumRuntime.CesiumGeoreference"))
  (Default|UpdateUI (Variables|Default|GetUIController) 0.0 0.0 0.0 0.0 0.0 (Variables|Default|GetFlightTimeSeconds) (Variables|Default|GetThreatBandStartAngle) (Variables|Default|GetThreatBandEndAngle) (Variables|Default|GetThreatBandThreatLevel) _outactors "0, 0, 0" "0, 0, 0" "0, 0, 0" "0, 0, 0" false))

(fn ConstructionScript)