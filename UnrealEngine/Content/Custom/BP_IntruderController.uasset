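; Replays recorded intruder traffic from a data table as on-screen arrow widgets.
; A self-recalling, delay-timed loop reads rows in timestamp pace, creating or refreshing widgets in a map keyed by identifier.
; Update separately maps longitude/latitude linearly onto the viewport from corner coordinates, removing intruders unseen for five seconds or holding last positions.
; GetClosestIntruderData, despite its name, keeps the largest distance and uses longitude for both X and Y.
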(event Custom|Activate
  (params (IntruderTable :type Data%20Table%20Object%20Reference))
  ;[1 1 1] Begin Update Loop
  (Variables|Default|SetIntruderTable IntruderTable)
  (CallFunction|UpdateLoop (Variables|Default|GetCurrentRow)))

(event Custom|UpdateLoop
  (params (Index :type Integer))
  ;[1 1 1] Update loop simply sets the values of the intruders -- does not actually set their position -- see `Update`
  (bind _returnvalue (Utilities|GetDataTableRow (Variables|Default|GetIntruderTable) (Utilities|String|StringToName (Utilities|String|ToString(Integer) Index)))
    (:then
      (if (.ReturnValue (Utilities|Map|Find (Variables|Default|GetIntruderMap) (.unique_identifier (Utilities|Struct|BreakStructure_Intruder _returnvalue))))
        (Default|UpdateValues (.Value (Utilities|Map|Find (Variables|Default|GetIntruderMap) (.unique_identifier (Utilities|Struct|BreakStructure_Intruder _returnvalue)))) (.timestamp (Utilities|Struct|BreakStructure_Intruder _returnvalue)) (.lon_degrees (Utilities|Struct|BreakStructure_Intruder _returnvalue)) (.lat_degrees (Utilities|Struct|BreakStructure_Intruder _returnvalue)) (.altitude_feet (Utilities|Struct|BreakStructure_Intruder _returnvalue)) (.heading_degrees (Utilities|Struct|BreakStructure_Intruder _returnvalue)))
        (else
          ;;[1 1 1] If Intruder has not been plotted yet
          (bind _returnvalue_2 (UserInterface|CreateWidget "/Game/Custom/UIComponentBlueprints/WBP_Intruder_Arrow.WBP_Intruder_Arrow_C"))
          (Utilities|Map|Add (Variables|Default|GetIntruderMap) (.unique_identifier (Utilities|Struct|BreakStructure_Intruder _returnvalue)) _returnvalue_2)
          (Default|Initialize _returnvalue_2 (.unique_identifier (Utilities|Struct|BreakStructure_Intruder _returnvalue)) (.timestamp (Utilities|Struct|BreakStructure_Intruder _returnvalue)) (.lon_degrees (Utilities|Struct|BreakStructure_Intruder _returnvalue)) (.lat_degrees (Utilities|Struct|BreakStructure_Intruder _returnvalue)) (.altitude_feet (Utilities|Struct|BreakStructure_Intruder _returnvalue)) (.heading_degrees (Utilities|Struct|BreakStructure_Intruder _returnvalue)))))
      (Utilities|FlowControl|Delay (/ (Math|Conversions|ToFloat(Integer) (.timestamp_delta (Utilities|Struct|BreakStructure_Intruder _returnvalue))) 1e+03)) ; Delay to maintain temporal consistency
      (Variables|Default|SetElapsedTime (.timestamp (Utilities|Struct|BreakStructure_Intruder _returnvalue)))
      (bind _result (Math|Integer|IncrementInt (Variables|Default|GetCurrentRow))
        (:%20%20
          (CallFunction|UpdateLoop _result))))
    (:RowNotFound
      (Development|PrintString "Intruder Row not found"))))

(event Custom|Update
  (params (TopLeftCoords :type Vector) (TopRightCoords :type Vector) (BottomRightCoords :type Vector) (OwnshipAltitude :type Float%20%28double-precision%29) (UseLast :type Boolean))
  ;[1 1 1] Using the location values stored in each intruder widget update their location and altitude difference on screen. If use last is true, simply maintain location on screen using previous values
  (bind _values (Utilities|Map|Values (Variables|Default|GetIntruderMap)))
  (for _array_element _values
    (if (not UseLast)
      (if (< (- (Variables|Default|GetElapsedTime) (Variables|/Game/Custom/UIComponentBlueprints/WBP_Intruder_Arrow.WBP_Intruder_Arrow_C|GetLastSeen%28ms%29 _array_element)) 5000)
        ;;[1 1 1] Use most current values in intruder -- Update position on screen
        (bind (_xpos _ypos) (CallFunction|CalculateIntruderScreenPosition TopLeftCoords TopRightCoords BottomRightCoords (Variables|/Game/Custom/UIComponentBlueprints/WBP_Intruder_Arrow.WBP_Intruder_Arrow_C|GetLongitude _array_element) (Variables|/Game/Custom/UIComponentBlueprints/WBP_Intruder_Arrow.WBP_Intruder_Arrow_C|GetLatitude _array_element)))
        (Default|Update _array_element _xpos _ypos OwnshipAltitude true)
        (else
          ;;[1 1 1] If intruder has not been seen in 5 seconds or more, remove it
          (Default|Disable _array_element)
          (Utilities|Map|Remove (Variables|Default|GetIntruderMap) (Variables|/Game/Custom/UIComponentBlueprints/WBP_Intruder_Arrow.WBP_Intruder_Arrow_C|GetIdentifier _array_element))))
      (else
        ;;[1 1 1] Use last values in intruder -- maintain position on screen
        (bind (_xpos_2 _ypos_2) (CallFunction|CalculateIntruderScreenPosition TopLeftCoords TopRightCoords BottomRightCoords (Variables|/Game/Custom/UIComponentBlueprints/WBP_Intruder_Arrow.WBP_Intruder_Arrow_C|GetLastLongitude _array_element) (Variables|/Game/Custom/UIComponentBlueprints/WBP_Intruder_Arrow.WBP_Intruder_Arrow_C|GetLastLatitude _array_element)))
        (Default|Update _array_element _xpos_2 _ypos_2 OwnshipAltitude false)))))

(fn ConstructionScript)

(fn CalculateIntruderScreenPosition
  (params (TopLeftCoords :type Vector) (TopRightCoords :type Vector) (BottomRightCoords :type Vector) (IntruderLongitude :type Float%20%28double-precision%29) (IntruderLatitude :type Float%20%28double-precision%29))
  (bind _x (Math|Vector|BreakVector TopLeftCoords))
  (bind (_x_2 _y) (Math|Vector|BreakVector TopRightCoords))
  (bind _returnvalue (Viewport|GetViewportSize))
  (bind (_x_3 _y_2) (Math|Vector2D|BreakVector2D _returnvalue))
  (return (* (/ (- IntruderLongitude _x) (- _x_2 _x)) _x_3) (* _y_2 (/ (- IntruderLatitude _y) (- (.Y (Math|Vector|BreakVector BottomRightCoords)) _y)))))

(fn GetClosestIntruderData
  (params (OwnshipLongLatHeight :type Vector))
  (Variables|Default|SetClosestIntruderDistance -1.0)
  (bind _values (Utilities|Map|Values (Variables|Default|GetIntruderMap)))
  (for _array_element _values
    (if (> (Math|Vector|Distance(Vector) (Math|Vector|MakeVector (Variables|/Game/Custom/UIComponentBlueprints/WBP_Intruder_Arrow.WBP_Intruder_Arrow_C|GetLastLongitude _array_element) (Variables|/Game/Custom/UIComponentBlueprints/WBP_Intruder_Arrow.WBP_Intruder_Arrow_C|GetLastLongitude _array_element) (Variables|/Game/Custom/UIComponentBlueprints/WBP_Intruder_Arrow.WBP_Intruder_Arrow_C|GetLastAltitude _array_element)) OwnshipLongLatHeight) (Variables|Default|GetClosestIntruderDistance))
      (Variables|Default|SetClosestIntruderDistance (Math|Vector|Distance(Vector) (Math|Vector|MakeVector (Variables|/Game/Custom/UIComponentBlueprints/WBP_Intruder_Arrow.WBP_Intruder_Arrow_C|GetLastLongitude _array_element) (Variables|/Game/Custom/UIComponentBlueprints/WBP_Intruder_Arrow.WBP_Intruder_Arrow_C|GetLastLongitude _array_element) (Variables|/Game/Custom/UIComponentBlueprints/WBP_Intruder_Arrow.WBP_Intruder_Arrow_C|GetLastAltitude _array_element)) OwnshipLongLatHeight))
      (Variables|Default|SetClosestIntruder _array_element)))
  (if (Utilities|IsValid (Variables|Default|GetClosestIntruder))
    (return (Variables|/Game/Custom/UIComponentBlueprints/WBP_Intruder_Arrow.WBP_Intruder_Arrow_C|GetLastHeading _array_element) (Variables|Default|GetClosestIntruderDistance) true)
    (else
      (return 0.0 0.0 false))))