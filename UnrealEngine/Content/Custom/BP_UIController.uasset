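; BP_UIController manages the active flight display widget, which receives ownship state, threat bands and intruder data.
; SetUI disables any active display, then creates and initializes the selected widget hidden in the viewport; only WBP_UIDesign_11 is wired.
; ToggleUI flips visibility, while UpdateUI forwards flight, threat, corner-coordinate and debug data to the widget.
; The widget is held in two references: ActiveUIObject for validity and visibility, ActiveUI for display calls.
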(event EventBeginPlay)

(fn ConstructionScript)

(fn SetUI
  (params (Selection :type Integer))
  (if (Utilities|IsValid (Variables|Default|GetActiveUIObject))
    (Default|Disable (Variables|Default|GetActiveUI)))
  (switch int Selection
    (:0
      (bind _returnvalue (UserInterface|CreateWidget "/Game/Custom/WBP_UIDesign_11.WBP_UIDesign_11_C" (Game|GetPlayerController 0)))
      (Variables|Default|SetActiveUI _returnvalue)
      (UserInterface|Viewport|AddtoViewport _returnvalue 0)
      (Variables|Default|SetActiveUIObject _returnvalue)
      (Default|Initialize _returnvalue)
      (Variables|/Script/UMG.Widget|SetVisibility _returnvalue "Hidden"))))

(fn ToggleUI
  (bind _activeuiobject (Variables|Default|GetActiveUIObject))
  (if (Utilities|IsValid (Variables|Default|GetActiveUIObject))
    (if (Widget|IsVisible _activeuiobject)
      (Widget|SetVisibility _activeuiobject "Hidden")
      (else
        (Widget|SetVisibility _activeuiobject "Visible")))))

(fn UpdateUI
  (params (OwnshipHeading :type Float%20%28double-precision%29) (OwnshipAltitude :type Float%20%28double-precision%29) (OwnshipGroundSpeed :type Float%20%28double-precision%29) (OwnshipRoll :type Float%20%28double-precision%29) (OwnshipPitch :type Float%20%28double-precision%29) (FlightTime :type Float%20%28double-precision%29) (ThreatBandStartAngle :type Float%20%28double-precision%29) (ThreatBandEndAngle :type Float%20%28double-precision%29) (ThreatBandThreatLevel :type Integer) (Intruders :type Array%20of%20BP%20Intruder%20Object%20References) (TopLeftCoord :type Vector) (TopRightCoord :type Vector) (BottomRightCoord :type Vector) (BottomLeftCoord :type Vector) (Debug :type Boolean))
  (if (Utilities|IsValid (Variables|Default|GetActiveUIObject))
    (Default|UpdateUI (Variables|Default|GetActiveUI) OwnshipHeading OwnshipAltitude OwnshipGroundSpeed OwnshipRoll OwnshipPitch FlightTime ThreatBandStartAngle ThreatBandEndAngle ThreatBandThreatLevel Intruders TopLeftCoord TopRightCoord BottomRightCoord BottomLeftCoord Debug)))